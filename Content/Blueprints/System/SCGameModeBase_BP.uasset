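; Game mode Blueprint for what appears to be an RTS, handing each joining player a starting group of workers.
; On PostLogin it increments a player counter and spawns a row of Worker2 actors, offset per player.
; Each valid worker is linked to that player's SCPlayerController and SCPlayerState.
; Disconnected leftover logic would assign existing unit-type selectables to the first player and create the HUD, but never runs.
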(event `self.K2_PostLogin`
  (params (NewPlayer :type "PlayerController Object Reference"))
  (bind _result (`/Engine/EditorBlueprintResources/StandardMacros.IncrementInt` (`self.num`))
    (:`  `
      (for _index (range 5)
        (bind _returnvalue (`|SpawnActorFromClass` "/Game/Blueprints/Units/Worker2.Worker2_C" (`KismetMathLibrary.MakeTransform` (`KismetMathLibrary.MakeVector` (`KismetMathLibrary.Conv_IntToDouble` (* _index 100)) (`KismetMathLibrary.Conv_IntToDouble` (* _result 200)) 40.0)) "AlwaysSpawn" "OverrideRootScale" null null))
        (if (`KismetSystemLibrary.IsValid` _returnvalue)
          (bind _asscplayer_controller (cast `SCPlayerController` NewPlayer))
          (`SCSelectable.SetPlayerController` _returnvalue _asscplayer_controller)
          (bind _asscplayer_state (cast `SCPlayerState` (`Controller.PlayerState` _asscplayer_controller)))
          (`SCSelectable.SetPlayerState` _returnvalue _asscplayer_state))))))

(fn `UserConstructionScript`)